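; BP_Bullet is a projectile that plays a shot sound on spawn and flies in straight or diagonal directions in the XZ plane.
; BeginPlay converts the vertical and horizontal direction signs into a Speed-scaled vector, then assigns it as the ProjectileMovement velocity.
; The capsule overlap destroys the bullet on contact with anything except its instigator or another bullet of the same class, without applying damage.
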(event OnComponentBeginOverlap(Capsule)
  (params (OverlappedComponent :type Primitive%20Component%20Object%20Reference) (OtherActor :type Actor%20Object%20Reference) (OtherComp :type Primitive%20Component%20Object%20Reference) (OtherBodyIndex :type Integer) (bFromSweep :type Boolean) (SweepResult :type Hit%20Result%20Structure%20%28by%20ref%29))
  (if (and (!= OtherActor (Game|GetInstigator)) (!= (Utilities|GetClass OtherActor) (Utilities|GetClass self)))
    (Actor|DestroyActor)))

(event EventBeginPlay
  (Audio|PlaySound2D "/Game/Bullets/shot.shot" 1.0 1.0 0.0 0 0)
  (Utilities|FlowControl|Sequence
    (:then_0
      (switch int (Variables|Default|GetverticalDirection)
        (:-1
          (Class|KismetMathLibrary|VectorSet (Variables|Default|Getdirection) 0.0 0.0 (* (Variables|Default|Getspeed) -1.0)))
        (:1
          (Class|KismetMathLibrary|VectorSet (Variables|Default|Getdirection) 0.0 0.0 (Variables|Default|Getspeed)))))
    (:then_1
      (switch int (Variables|Default|GethorizontalDirection)
        (:-1
          (Class|KismetMathLibrary|VectorSet (Variables|Default|Getdirection) (* (Variables|Default|Getspeed) -1.0) 0.0 (.z (Variables|Default|Getdirection))))
        (:1
          (Class|KismetMathLibrary|VectorSet (Variables|Default|Getdirection) (Variables|Default|Getspeed) 0.0 (.z (Variables|Default|Getdirection))))))
    (:then_2
      (Variables|/Script/Engine.MovementComponent|SetVelocity (Variables|Default|GetProjectileMovement) (Variables|Default|Getdirection)))))

(fn ConstructionScript)