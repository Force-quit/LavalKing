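; BP_Spider is an enemy spider that chases the player and can be damaged and killed.
; BeginPlay sends a move message, and the Move event runs AI MoveTo toward the player, re-issuing it after a short delay on success or failure.
; Hit subtracts the incoming power from health and triggers Die at zero or below, which plays a 2D death sound and destroys the actor.
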(event EventBeginPlay
  (Class|IEnemy|Move(Message) self))

(event EventMove
  (AI|AIMoveTo self "0, 0, 0" (Variables|Default|Getplayer) 1e+01 false
    (:OnSuccess
      _)
    (:OnFail
      _))
  (Utilities|FlowControl|Delay 0.2)
  (CallFunction|Move))

(event EventDie
  (Audio|PlaySound2D "/Game/Enemies/Maniac/Maniac_death.Maniac_death" 1.0 1.0 0.0 0 0)
  (Actor|DestroyActor))

(event EventHit
  (params (power :type Integer))
  (bind _output_get (Variables|Default|Sethealth (- (Variables|Default|Gethealth) power)))
  (if (<= _output_get 0)
    (CallFunction|Die)))

(fn ConstructionScript)