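; BP_Maniac is a wandering enemy that takes damage and dies.
; BeginPlay sends a Move message, and the Move event uses AIMoveTo to roam to random reachable navmesh points around itself.
; It loops by calling Move again, after a short delay on success or immediately on failure, with debug prints on both.
; Hit subtracts Power from Health and triggers Die at zero or below, which plays a death sound and destroys the actor.
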(event EventBeginPlay
  (Class|IEnemy|Move(Message) self))

(event EventMove
  (AI|AIMoveTo self (.RandomLocation (AI|Navigation|GetRandomReachablePointinRadius (Transformation|GetActorLocation) 1e+03 (Variables|Default|GetNavData) "/Script/AIModule.NavFilter_AIControllerDefault")) 0 5.0 false
    (:OnSuccess
      (Development|PrintString "YES")
      (Utilities|FlowControl|Delay 0.2))
    (:OnFail
      (Development|PrintString "Hello")))
  (CallFunction|Move))

(event EventDie
  (Audio|PlaySound2D "/Game/Enemies/Maniac/Maniac_death.Maniac_death" 1.0 1.0 0.0 0 0)
  (Actor|DestroyActor))

(event EventHit
  (params (power :type Integer))
  (bind _output_get (Variables|Default|SetHealth (- (Variables|Default|GetHealth) power)))
  (if (<= _output_get 0)
    (CallFunction|Die)))

(fn ConstructionScript)