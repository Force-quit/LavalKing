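; BP_Spider is a spider NPC that continually chases the player through AI navigation.
; From BeginPlay, MoveNPC finds the BP_Player actor and issues AIMoveTo to a random reachable point within a small radius of its location.
; On either success or failure, it waits briefly and calls itself again, so each new move samples the player's position afresh.
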(event Custom|Move%20NPC
  (bind _returnvalue (Actor|GetActorOfClass "/Game/Player/BP_Player.BP_Player_C"))
  (AI|AIMoveTo self (.RandomLocation (AI|Navigation|GetRandomReachablePointinRadius (Transformation|GetActorLocation _returnvalue) 1e+01 (Variables|Default|GetNavData) 0)) 0 5.0 false
    (:OnSuccess
      (Utilities|FlowControl|Delay 0.2)
      (CallFunction|MoveNPC))
    (:OnFail
      (Utilities|FlowControl|Delay 0.2)
      (CallFunction|MoveNPC))))

(event EventBeginPlay
  (CallFunction|MoveNPC))

(fn ConstructionScript)