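; BP_Player is the player actor, which moves in the world X/Z plane and fires bullets.
; On BeginPlay it adds the IM_Default Enhanced Input mapping context to its player controller.
; IA_Move feeds movement input along X and Z.
; IA_Fire spawns a BP_Bullet at the player's transform on each trigger, passing the input axes truncated to integer directions and itself as instigator.
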(event Input|EnhancedActionEvents|EnhancedInputActionIA_Move
  (params (ActionValue :type Vector%202D%20Structure) (ElapsedSeconds :type Float%20%28double-precision%29) (TriggeredSeconds :type Float%20%28double-precision%29) (InputAction :type Input%20Action%20Object%20Reference :default "/Game/Inputs/IA_Move.IA_Move"))
  (:Triggered
    (Pawn|Input|AddMovementInput (Math|Vector|MakeVector (.x ActionValue) 0.0 (.y ActionValue)) 1.0 false)))

(event Input|EnhancedActionEvents|EnhancedInputActionIA_Fire
  (params (ActionValue :type Vector%202D%20Structure) (ElapsedSeconds :type Float%20%28double-precision%29) (TriggeredSeconds :type Float%20%28double-precision%29) (InputAction :type Input%20Action%20Object%20Reference :default "/Game/Inputs/IA_Fire.IA_Fire"))
  (:Triggered
    (Game|SpawnActorfromClass "/Game/Bullets/BP_Bullet.BP_Bullet_C" (Transformation|GetActorTransform) "Undefined" 0 (Math|Float|Truncate (.x ActionValue)) (Math|Float|Truncate (.y ActionValue)) self)))

(event EventBeginPlay
  (bind _asplayer_controller (Utilities|Casting|CastToPlayerController (Pawn|GetController)))
  (Input|AddMappingContext (PlayerController|LocalPlayerSubsystems|GetEnhancedInputLocalPlayerSubsystem _asplayer_controller) "/Game/Inputs/IM_Default.IM_Default" 0 "(bIgnoreAllPressedKeysUntilRelease=True,bForceImmediately=False)"))

(fn ConstructionScript)