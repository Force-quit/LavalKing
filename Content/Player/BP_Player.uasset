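; BP_Player is a flipbook-sprite player pawn that moves and shoots in eight directions via Enhanced Input, tracking score and lives.
; Firing asks BPShootingComponent for permission, then spawns BP_Bullet along the truncated stick direction.
; The same input resolves into a combined direction enum that selects the sprite's flipbook, including idle.
; Overlapping an I_Enemy kills it and costs a life, printing "Game over" when none remain.
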(event OnComponentBeginOverlap(CapsuleComponent)
  (params (OverlappedComponent :type Primitive%20Component%20Object%20Reference) (OtherActor :type Actor%20Object%20Reference) (OtherComp :type Primitive%20Component%20Object%20Reference) (OtherBodyIndex :type Integer) (bFromSweep :type Boolean) (SweepResult :type Hit%20Result%20Structure%20%28by%20ref%29))
  (bind _asi_enemy (Utilities|Casting|CastToI_Enemy OtherActor))
  (Default|Die _asi_enemy)
  (Variables|Default|Setlifes (- (Variables|Default|Getlifes) 1))
  (if (<= (Variables|Default|Getlifes) 0)
    (Development|PrintString "Game over")))

(event Custom|ComputeAnimation
  (params (fireX :type Integer) (fireY :type Integer))
  (Utilities|FlowControl|Sequence
    (:then_0
      (switch int fireX
        (:-1
          (Variables|Animation|SethorizontalShootingDirection "NewEnumerator2"))
        (:0
          (Variables|Animation|SethorizontalShootingDirection "NewEnumerator4"))
        (:1
          (Variables|Animation|SethorizontalShootingDirection "NewEnumerator3"))))
    (:then_1
      (switch int fireY
        (:-1
          (Variables|Animation|SetVerticalShootingDirection "NewEnumerator0"))
        (:0
          (Variables|Animation|SetVerticalShootingDirection "NewEnumerator4"))
        (:1
          (Variables|Animation|SetVerticalShootingDirection "NewEnumerator1"))))
    (:then_2
      (if (and (Utilities|Enum|Equal(Enum) (Variables|Animation|GethorizontalShootingDirection) "NewEnumerator2") (Utilities|Enum|Equal(Enum) (Variables|Animation|GetVerticalShootingDirection) "NewEnumerator0"))
        (Variables|Animation|SetcalculatedShootingDirection "NewEnumerator5")
        (elif (and (Utilities|Enum|Equal(Enum) (Variables|Animation|GethorizontalShootingDirection) "NewEnumerator2") (Utilities|Enum|Equal(Enum) (Variables|Animation|GetVerticalShootingDirection) "NewEnumerator1"))
          (Variables|Animation|SetcalculatedShootingDirection "NewEnumerator7")
          (elif (and (Utilities|Enum|Equal(Enum) (Variables|Animation|GethorizontalShootingDirection) "NewEnumerator3") (Utilities|Enum|Equal(Enum) (Variables|Animation|GetVerticalShootingDirection) "NewEnumerator0"))
            (Variables|Animation|SetcalculatedShootingDirection "NewEnumerator6")
            (elif (and (Utilities|Enum|Equal(Enum) (Variables|Animation|GethorizontalShootingDirection) "NewEnumerator3") (Utilities|Enum|Equal(Enum) (Variables|Animation|GetVerticalShootingDirection) "NewEnumerator1"))
              (Variables|Animation|SetcalculatedShootingDirection "NewEnumerator8")
              (elif (Utilities|Enum|Equal(Enum) (Variables|Animation|GethorizontalShootingDirection) "NewEnumerator4")
                (Variables|Animation|SetcalculatedShootingDirection (Variables|Animation|GetVerticalShootingDirection))
                (else
                  (Variables|Animation|SetcalculatedShootingDirection (Variables|Animation|GethorizontalShootingDirection)))))))))
    (:then_3
      (CallFunction|SetAnimation))))

(event Custom|SetAnimation
  (Sprite|SetFlipbook (Variables|Default|GetSprite) (Utilities|Select :Index (Variables|Animation|GetcalculatedShootingDirection) :NewEnumerator0 (Variables|Animation|GetTop) :NewEnumerator1 (Variables|Animation|GetDown) :NewEnumerator2 (Variables|Animation|GetLeft) :NewEnumerator3 (Variables|Animation|GetRight) :NewEnumerator4 (Variables|Animation|GetIdle) :NewEnumerator5 (Variables|Animation|GetTopLeft) :NewEnumerator6 (Variables|Animation|GetTopRight) :NewEnumerator7 (Variables|Animation|GetBottomLeft) :NewEnumerator8 (Variables|Animation|GetBottomRight))))

(event Custom|AddScore
  (Variables|Default|Setscore (+ (Variables|Default|Getscore) 1)))

(event Input|EnhancedActionEvents|EnhancedInputActionIA_Move
  (params (ActionValue :type Vector%202D%20Structure) (ElapsedSeconds :type Float%20%28double-precision%29) (TriggeredSeconds :type Float%20%28double-precision%29) (InputAction :type Input%20Action%20Object%20Reference :default "/Game/Inputs/IA_Move.IA_Move"))
  (:Triggered
    (Pawn|Input|AddMovementInput (Math|Vector|MakeVector (.x ActionValue) (.y ActionValue) 0.0) 1.0 false)))

(event Input|EnhancedActionEvents|EnhancedInputActionIA_Fire
  (params (ActionValue :type Vector%202D%20Structure) (ElapsedSeconds :type Float%20%28double-precision%29) (TriggeredSeconds :type Float%20%28double-precision%29) (InputAction :type Input%20Action%20Object%20Reference :default "/Game/Inputs/IA_Fire.IA_Fire"))
  (bind _returnvalue (Math|Float|Truncate (.x ActionValue)))
  (bind _returnvalue_2 (* (.y ActionValue) -1.0))
  (bind _returnvalue_3 (Math|Float|Truncate _returnvalue_2))
  (:Triggered
    (Utilities|FlowControl|Sequence
      (:then_0
        (bind _canshoot (Default|TryShoot (Variables|Default|GetBP_Shooting_Component)))
        (if _canshoot
          (Game|SpawnActorfromClass "/Game/Bullets/BP_Bullet.BP_Bullet_C" (Transformation|GetActorTransform) "Undefined" 0 _returnvalue _returnvalue_3 1 self)))
      (:then_1
        (CallFunction|ComputeAnimation _returnvalue _returnvalue_3 :!label _label))))
  (:Completed
    (goto _label)))

(event EventBeginPlay
  (bind _asplayer_controller (Utilities|Casting|CastToPlayerController (Pawn|GetController)))
  (Input|AddMappingContext (PlayerController|LocalPlayerSubsystems|GetEnhancedInputLocalPlayerSubsystem _asplayer_controller) "/Game/Inputs/IM_Default.IM_Default" 0 "(bIgnoreAllPressedKeysUntilRelease=True,bForceImmediately=False)"))

(fn ConstructionScript)